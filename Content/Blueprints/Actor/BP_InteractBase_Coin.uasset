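; BP_InteractBase_Coin is a coin pickup actor that a player collects by interacting with it.
; Its Interact function adds one to the player's Coins, decrements CoinsLeft on B_BWJGameGameModeBase, plays a 2D coin sound, then destroys the actor.
; If the game mode cast fails, the player still gains the coin, but the sound and destruction are skipped.
; The event graph holds only disabled default events.
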(event EventBeginPlay
  (|CallParentFunction) ; This node is disabled and will not be called.\nDrag off pins to build functionality.
)

(event Collision|EventActorBeginOverlap
  (params (OtherActor :type Actor%20Object%20Reference)))

(event EventTick
  (params (DeltaSeconds :type Float%20%28single-precision%29)))

(fn ConstructionScript
  (|CallParentFunction))

(fn Interact
  (params (PlayerRef :type BP%20Player%20Base%20Object%20Reference))
  (Variables|/Game/Blueprints/Character/BP_PlayerBase.BP_PlayerBase_C|SetCoins PlayerRef (+ (Variables|/Game/Blueprints/Character/BP_PlayerBase.BP_PlayerBase_C|GetCoins PlayerRef) 1))
  (bind _asb_bwjgame_game_mode_base (Utilities|Casting|CastToB_BWJGameGameModeBase (Game|GetGameMode)))
  (bind _result (Math|Integer|DecrementInt (Variables|/Game/Blueprints/GameModes/B_BWJGameGameModeBase.B_BWJGameGameModeBase_C|GetCoins%20Left _asb_bwjgame_game_mode_base))
    (:%20%20
      (Variables|/Game/Blueprints/GameModes/B_BWJGameGameModeBase.B_BWJGameGameModeBase_C|SetCoins%20Left _asb_bwjgame_game_mode_base _result)
      (Audio|PlaySound2D "/Game/Sounds/Cues/Coin_Cue.Coin_Cue" 1.0 1.0 0.0 0 0)
      (Actor|DestroyActor))))