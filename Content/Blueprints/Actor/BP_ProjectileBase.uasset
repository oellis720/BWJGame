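; Base projectile actor that damages player characters on contact and expires once it travels beyond its range.
; BeginPlay records the start location, and Tick destroys the projectile when its distance from that point reaches ProjectileRange.
; Sphere overlaps with a BP_PlayerBase apply Damage and destroy the projectile, while other actors are ignored.
; Separate DoOnce gates keep the hit and range expiry from repeating.
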(event OnComponentBeginOverlap(Sphere)
  (params (OverlappedComponent :type Primitive%20Component%20Object%20Reference) (OtherActor :type Actor%20Object%20Reference) (OtherComp :type Primitive%20Component%20Object%20Reference) (OtherBodyIndex :type Integer) (bFromSweep :type Boolean) (SweepResult :type Hit%20Result%20Structure%20%28by%20ref%29))
  ;[1 1 1] Applies damage to player character
  (bind _asbp_player_base (Utilities|Casting|CastToBP_PlayerBase OtherActor))
  (Utilities|FlowControl|DoOnce false
    (:Completed
      (Game|Damage|ApplyDamage _asbp_player_base (Variables|Default|GetDamage) 0 self)
      (Actor|DestroyActor))))

(event EventBeginPlay
  (Variables|Default|SetStartLocation (Transformation|GetActorLocation)))

(event Collision|EventActorBeginOverlap
  (params (OtherActor :type Actor%20Object%20Reference)))

(event EventTick
  (params (DeltaSeconds :type Float%20%28single-precision%29))
  ;[1 1 1] destroys projectile based on range
  (if (>= (Math|Vector|VectorLength (- (Variables|Default|GetStartLocation) (Transformation|GetActorLocation))) (Variables|Default|GetProjectileRange))
    (Utilities|FlowControl|DoOnce false
      (:Completed
        (Actor|DestroyActor)))))

(fn ConstructionScript)