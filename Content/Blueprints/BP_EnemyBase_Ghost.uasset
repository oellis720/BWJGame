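; Ghost enemy base that shoots projectiles at players and destroys itself on death.
; Each tick it targets the nearest player pawn within SenseRange; a line-of-sight check runs, but the following branch is hardwired true.
; UpdateFire calls Fire once the RateOfFire cooldown passes and a dot product shows the capsule facing the target.
; Fire spawns a projectile at the sprite's socket, gated by a DoN that resets after a short delay.
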(event Custom|Fire
  (Variables|Private|SetTimeDelayFire (Utilities|Time|GetGameTimeinSeconds))
  (Utilities|FlowControl|Sequence
    (:then_0
      (goto _label Reset))
    (:then_1
      (Utilities|FlowControl|DoN 1 :!label _label
        (:Exit
          (Game|SpawnActorfromClass "/Game/Blueprints/BP_ProjectileBase.BP_ProjectileBase_C" (Transformation|GetSocketTransform (Variables|Default|GetSprite) "Projectile" "RTS_World") "Undefined" 0 0)
          (Utilities|FlowControl|Delay 0.2)
          (goto _label Reset))))))

(event EventBeginPlay)

(event Collision|EventActorBeginOverlap
  (params (OtherActor :type Actor%20Object%20Reference)))

(event EventTick
  (params (DeltaSeconds :type Float%20%28single-precision%29))
  (CallFunction|FindTarget)
  (Variables|Private|GetTarget
    (:then
      (CallFunction|UpdateFire))
    (:else)))

(fn ConstructionScript
  (|CallParentFunction))

(fn FindTarget
  (LocalVariables|SetBestDistanceLocal (+ (Variables|Const|GetSenseRange) 1.0))
  (bind _outactors (Collision|SphereOverlapActors (Transformation|GetActorLocation) (Variables|Const|GetSenseRange) (Utilities|Array|MakeArray "ObjectTypeQuery3") "/Game/Blueprints/BP_PlayerBase.BP_PlayerBase_C"))
  (for _array_element _outactors
    (bind _output_get (LocalVariables|SetCurrentTargetLocal _array_element))
    (bind _output_get_2 (LocalVariables|SetCurrentDistanceLocal (Transformation|GetDistanceTo _output_get self)))
    (if (or (< _output_get_2 (LocalVariables|GetBestDistanceLocal)) (not (Utilities|IsValid (LocalVariables|GetBestTargetLocal))))
      (CallFunction|LineOfSight (Transformation|GetWorldLocation (Variables|Default|GetCapsuleComponent)) (Transformation|GetActorLocation (LocalVariables|GetCurrentTargetLocal)) (Utilities|Array|MakeArray self (LocalVariables|GetCurrentTargetLocal)))
      (if true
        (LocalVariables|SetBestTargetLocal (LocalVariables|GetCurrentTargetLocal))
        (LocalVariables|SetBestDistanceLocal (LocalVariables|GetCurrentDistanceLocal)))))
  (Variables|Private|SetTarget (LocalVariables|GetBestTargetLocal)))

(fn UpdateFire
  (if (> (- (Utilities|Time|GetGameTimeinSeconds) (Variables|Private|GetTimeDelayFire)) (Variables|Const|GetRate%20of%20fire)) ; rof cooldown?
    (if (> (Math|Vector|DotProduct (Math|Vector|GetUnitDirection(Vector) (Transformation|GetWorldLocation (Variables|Default|GetCapsuleComponent)) (Transformation|GetActorLocation (Variables|Private|GetTarget))) (Math|Vector|GetForwardVector (Variables|Default|GetCapsuleComponent))) 0.99) ; turret facing target
      (CallFunction|Fire))))

(fn EnemyDied
  (|CallParentFunction)
  (Actor|DestroyActor))